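; BPA_BasicEnvironment is an environment actor that exposes time-of-day and date control through a referenced SunSky.
; SetSolarTime and SetDate write solar time, day and month to SunSky after a validity check, while GetSolarTime reads the time back or returns zero.
; Weather is unsupported: GetAvailableWeather supplies no options and GetWeather always returns UNDEFINED.
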(event `self.ReceiveBeginPlay`)

(event `GenericTwinEnvControlInterface.SetSolarTime`
  (params (SolarTime :type "Float (single-precision)"))
  (bind _sunsky (`self.SunSky`)
    (:`then`
      (set `/SunPosition/SunSky.SolarTime` SolarTime _sunsky))
    (:`else`)))

(event `GenericTwinEnvControlInterface.SetDate`
  (params (Day :type Integer) (Month :type Integer) (Year :type Integer))
  (if (`KismetSystemLibrary.IsValid` (`self.SunSky`))
    (set `/SunPosition/SunSky.Day` Day (`self.SunSky`))
    (set `/SunPosition/SunSky.Month` Month (`self.SunSky`))))

(fn `GetAvailableWeather`
  (returns (ReturnValue :type "Array of EGenericTwinWeatherType Enum"))
  (return))

(fn `GetSolarTime`
  (returns (ReturnValue :type "Float (single-precision)"))
  (if (`KismetSystemLibrary.IsValid` (`self.SunSky`))
    (return (`/SunPosition/SunSky.SolarTime` (`self.SunSky`)))
    (else
      (return 0.0))))

(fn `GetWeather`
  (returns (ReturnValue :type "EGenericTwinWeatherType Enum"))
  (return "UNDEFINED"))

(fn `UserConstructionScript`)